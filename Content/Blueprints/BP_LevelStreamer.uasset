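; Level streamer actor that switches between the main menu and three table levels by loading and unloading streaming sublevels.
; A bound RealStreamLevel event maps the requested name to a sublevel list, with table levels sharing a base level plus their own dynamic level.
; For valid names, loops unload active levels absent from that list, then load each listed level with blocking calls, updating the active-level array.
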(event `self.ReceiveTick`
  (params (DeltaSeconds :type "Float (single-precision)")))

(event `self.ReceiveBeginPlay`
  (add `self.RealStreamLevel` (delegate `RealStreamLevel_Event`))
  (`KismetArrayLibrary.Array_Add` (`self.ActiveLevels`) "MainMenu"))

(event `RealStreamLevel_Event` :!signature `self.RealStreamLevel`
  (params (LevelName :type Name))
  (bind _index (`self.Index`))
  (bind _activelevels (`self.ActiveLevels`))
  (bind _index_2 (`self.Index`))
  (bind _levelstoload (`self.LevelsToLoad`))
  (bind _output (`|GetArrayItem` _levelstoload _index))
  (bind _output_2 (`|GetArrayItem` _activelevels _index_2))
  (set `self.IsLevelNameValid` true)
  (`KismetSystemLibrary.PrintString` (`KismetStringLibrary.Concat_StrStr` "Loads level " (`KismetStringLibrary.Conv_NameToString` "None")) false)
  (`|ExecutionSequence`
    (:`then_0`
      (`KismetArrayLibrary.Array_Clear` (`self.LevelsToLoad`))
      (switch `name` LevelName
        (:`Default`
          (`KismetSystemLibrary.PrintString` "No level set with the specified name" true true (struct :`R` 1.0 :`B` 0.02001 :`A` 1.0) 10.0)
          (set `self.IsLevelNameValid` false))
        (:`TableLevel01`
          ;[1 1 1] TableLevel01
          (set `self.LevelsToLoad` (`|MakeArray` "BaseTableLevel" "TableDynamicOnly")))
        (:`TableLevel02`
          ;[1 1 1] TableLevel02
          (set `self.LevelsToLoad` (`|MakeArray` "BaseTableLevel" "TableDynamicOnly2")))
        (:`TableLevel03`
          ;[1 1 1] TableLevel03
          (set `self.LevelsToLoad` (`|MakeArray` "BaseTableLevel" "TableDynamicOnly3")))
        (:`MainMenu`
          ;[1 1 1] MainMenu
          (set `self.LevelsToLoad` (`|MakeArray` "MainMenu")))))
    (:`then_1`
      (if (`self.IsLevelNameValid`)
        ;[1 1 1] Unload unnecessary levels.
        (if (> (`KismetArrayLibrary.Array_Length` _activelevels) _index_2) :!label _label
          (if (`KismetArrayLibrary.Array_Contains` (`self.LevelsToLoad`) _output_2)
            (`/Engine/EditorBlueprintResources/StandardMacros.IncrementInt` (`self.Index`)
              (:`  `
                (goto _label)))
            (else
              (`GameplayStatics.UnloadStreamLevel` _output_2 true)
              (`KismetArrayLibrary.Array_RemoveItem` (`self.ActiveLevels`) _output_2)
              (goto _label)))
          (else
            (set `self.Index` 0)
            (`KismetSystemLibrary.PrintString` "Finished unload" false)
            ;[1 1 1] Load necessary levels.
            (if (> (`KismetArrayLibrary.Array_Length` _levelstoload) _index) :!label _label_2
              (`GameplayStatics.LoadStreamLevel` _output true true)
              (`KismetArrayLibrary.Array_Add` (`self.ActiveLevels`) _output)
              (`KismetArrayLibrary.Array_RemoveItem` (`self.LevelsToLoad`) _output)
              (goto _label_2)
              (else
                (`KismetSystemLibrary.PrintString` "Finished load" false)))))))))

(fn `PrintArray`
  (params (Array :type "Array of Name (by ref)"))
  (locals (OutputString :type String))
  (set `local.OutputString` "")
  (for _array_element Array
    (set `local.OutputString` (`KismetStringLibrary.Concat_StrStr` (`local.OutputString`) ", " (`KismetStringLibrary.Conv_NameToString` _array_element))))
  (`KismetSystemLibrary.PrintString` (`local.OutputString`) false))

(fn `UserConstructionScript`)