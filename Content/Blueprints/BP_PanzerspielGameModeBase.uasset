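; Game mode for the local multiplayer tank game Panzerspiel that handles player setup, menus, pausing and level streaming.
; On BeginPlay it creates the additional local players, possesses tank pawns spawned at PlayerStarts tagged by player index, then shows the main menu.
; Level changes go through a BP_LevelStreamer found in the world, with its stream event relayed here so the persistent level could intercept it.
; Menu and pause widgets toggle player 0's cursor and input mode.
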(event `self.ReceiveBeginPlay`
  (`self.GetPlayerStartPoints`)
  (`self.CreatePlayers`)
  (bind _outactors (`GameplayStatics.GetAllActorsOfClass` "/Game/Blueprints/BP_LevelStreamer.BP_LevelStreamer_C"))
  (for _array_element _outactors
    (set `self.LevelStreamer` _array_element)
    (break))
  (`self.ShowMainMenu`))

(event `self.LevelStreamer.StreamLevel`
  (params (LevelName :type Name))
  ;[1 1 1] This way the persistent level could stop the event from firing if it would be necessary.
  (`KismetSystemLibrary.PrintString` "Called Stream level")
  (`/Game/Blueprints/BP_LevelStreamer.RealStreamLevel` (`self.LevelStreamer`) LevelName))

(event `Released P key`
  (`self.ShowPauseMenu`))

(fn `BackToMenu`
  (`GameplayStatics.SetGamePaused` false)
  (`Widget.RemoveFromParent` (`self.PauseMenu`))
  (`self.StreamLevelByName` "MainMenu")
  (`self.ShowMainMenu`))

(fn `CreatePlayers`
  (for _index (range 1 (`self.MaxPlayers`))
    (bind _output_get (set `self.PlayerIndex` _index))
    (`GameplayStatics.CreatePlayer` _output_get)
    (for _array_element (`self.PlayerStarts`)
      (if (== (`PlayerStart.PlayerStartTag` _array_element) (`KismetStringLibrary.Conv_StringToName` (`KismetStringLibrary.Conv_IntToString` _output_get)))
        (bind _returnvalue (`|SpawnActorFromClass` "/Game/Blueprints/BP_TankPawn.BP_TankPawn_C" (`self.GetTransform` _array_element) "AlwaysSpawn" "OverrideRootScale" null null))
        (`Controller.Possess` (`GameplayStatics.GetPlayerController` (`self.PlayerIndex`)) _returnvalue)))))

(fn `GetPlayerStartPoints`
  (bind _outactors (`GameplayStatics.GetAllActorsOfClass` "/Script/Engine.PlayerStart"))
  (set `self.PlayerStarts` _outactors))

(fn `HideMainMenu`
  (bind _returnvalue (`GameplayStatics.GetPlayerController` 0))
  (`Widget.RemoveFromParent` (`self.MainMenu`))
  (`WidgetBlueprintLibrary.SetInputMode_GameOnly` _returnvalue)
  (set `PlayerController.bShowMouseCursor` false _returnvalue))

(fn `ResumeGame`
  (bind _returnvalue (`GameplayStatics.GetPlayerController` 0))
  (bind _pausemenu (`self.PauseMenu`))
  (`/Engine/EditorBlueprintResources/StandardMacros.IsValid` _pausemenu
    (:`Is Valid`
      (`Widget.RemoveFromParent` _pausemenu)
      (set `PlayerController.bShowMouseCursor` false _returnvalue)
      (`WidgetBlueprintLibrary.SetInputMode_GameOnly` _returnvalue)
      (`GameplayStatics.SetGamePaused` false))))

(fn `ShowMainMenu`
  (bind _returnvalue (`GameplayStatics.GetPlayerController` 0))
  (`/Engine/EditorBlueprintResources/StandardMacros.IsValid` (`self.MainMenu`)
    (:`Is Valid`
      _)
    (:`Is Not Valid`
      (bind _returnvalue_2 (`|CreateWidget` "/Game/UI/MainMenu.MainMenu_C" null null))
      (set `self.MainMenu` _returnvalue_2)))
  (set `PlayerController.bShowMouseCursor` true _returnvalue)
  (`WidgetBlueprintLibrary.SetInputMode_UIOnlyEx` _returnvalue null)
  (`UserWidget.AddToViewport` (`self.MainMenu`) 0))

(fn `ShowPauseMenu`
  (bind _returnvalue (`GameplayStatics.GetPlayerController` 0))
  (`/Engine/EditorBlueprintResources/StandardMacros.IsValid` (`self.PauseMenu`)
    (:`Is Valid`
      _)
    (:`Is Not Valid`
      (bind _returnvalue_2 (`|CreateWidget` "/Game/UI/PauseMenu.PauseMenu_C" null null))
      (set `self.PauseMenu` _returnvalue_2)))
  (set `PlayerController.bShowMouseCursor` true _returnvalue)
  (`WidgetBlueprintLibrary.SetInputMode_UIOnlyEx` _returnvalue null)
  (`UserWidget.AddToViewport` (`self.PauseMenu`) 0)
  (`GameplayStatics.SetGamePaused` true))

(fn `StreamLevelByName`
  (params (LevelName :type Name))
  (`/Game/Blueprints/BP_LevelStreamer.RealStreamLevel` (`self.LevelStreamer`) LevelName)
  (`self.HideMainMenu`))

(fn `UserConstructionScript`)