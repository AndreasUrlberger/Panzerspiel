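; BP_TankAI is a tank AI Blueprint whose graph only handles the visual effect for an explosion.
; Its PlayNiagaraExplosion event spawns the Niagara explosion system at a supplied location.
; The rotation comes from a random 0–1 value in the vector's Y component, converted through a quaternion, although the node comment describes random rotation around the Z axis.
; BeginPlay, overlap and Tick are disabled stubs, and the construction script only calls its parent.
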(event `self.PlayNiagaraExplosion`
  (params (SpawnLocation :type "Vector Structure"))
  (`NiagaraFunctionLibrary.SpawnSystemAtLocation` (`self.NiagaraExplosionSystem`) SpawnLocation (`KismetMathLibrary.Quat_Rotator` (`KismetMathLibrary.Conv_VectorToQuaterion` (`KismetMathLibrary.MakeVector` 0.0 (`KismetMathLibrary.RandomFloat`))))))

(fn `UserConstructionScript`
  (`parent.UserConstructionScript`))